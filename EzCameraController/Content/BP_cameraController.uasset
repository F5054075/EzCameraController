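; Camera controller Blueprint that drives the player camera and switches the view to other cameras.
; BeginPlay caches player references and starts a Perlin shake; functions handle attachment, teleporting, rotation, input toggling and four timed shake types.
; Timelines scale play rate for smooth moves, rotations and turntable orbits, which spin a camera actor's root before switching back.
; A looping, pausable near-zero timer keeps the current camera facing the player.
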(event `self.ReceiveBeginPlay`
  (bind _returnvalue (`GameplayStatics.GetPlayerCharacter` 0))
  ; gets the player controller/character, the spring arm on the player and the players camera
  (set `self.playerController` (`GameplayStatics.GetPlayerController` 0))
  (set `self.playerCharacter` _returnvalue)
  (set `self.springArm` (`self.GetComponentByClass` _returnvalue "/Script/Engine.SpringArmComponent"))
  (bind _output_get (set `self.playerCamera` (`self.GetComponentByClass` _returnvalue "/Script/Engine.CameraComponent")))
  (set `self.currentCamera` _output_get)
  (`self.shakeCameraPerlin` 30.0 10.0))

(event `smoothMoveCameraToPoisiton`
  (params (endPos :type "Vector Structure") (howManySecondsTakes :type "Float (double-precision)"))
  ; moves the camera from its current position to a new one in a set amount of time
  (set `self.End PosForCamera` endPos)
  (set `self.orgionalCameraPos` (`SceneComponent.K2_GetComponentLocation` (`self.playerCamera`)))
  (`TimelineComponent.SetPlayRate` (`self.moveToPos`) (/ 1.0 howManySecondsTakes))
  (bind (_direction _a) (`Timeline|moveToPos` :!via `PlayFromStart`)
    (:`Update`
      (`SceneComponent.K2_SetWorldLocation` (`self.playerCamera`) (`KismetMathLibrary.VLerp` (`self.orgionalCameraPos`) (`self.End PosForCamera`) _a) false false))))

(event `smoothRotateCamera`
  (params (endRotation :type "Rotator Structure") (howManySecondsTakes :type "Float (double-precision)"))
  ; rotates the camera from its current rotation to a new one in a set amount of time
  (set `self.End RotationForCamera` endRotation)
  (set `self.startRotation` (`SceneComponent.K2_GetComponentRotation` (`self.playerCamera`)))
  (`TimelineComponent.SetPlayRate` (`self.rotateTo`) (/ 1.0 howManySecondsTakes))
  (bind (_direction _a) (`Timeline|rotateTo` :!via `PlayFromStart`)
    (:`Update`
      (`SceneComponent.K2_SetWorldRotation` (`self.playerCamera`) (`KismetMathLibrary.RLerp` (`self.startRotation`) (`self.End RotationForCamera`) _a) false false))))

(event `turnTableRotate`
  (params (speed :type "Float (double-precision)") (howLongToDoItFor :type "Float (double-precision)") (cameraToSwitchBackTo :type "CameraComponent Object Reference") (switchToPlayerCamera :type Boolean) (disablePlayerInput :type Boolean))
  ; rotates the cameras parent in a circle rotating the camera around the center of the object to show off whatever is in view from all angles
  (`TimelineComponent.SetPlayRate` (`self.turntableRotateTimeline`) speed)
  (bind (_direction _newtrack_0) (`Timeline|turntableRotateTimeline` :!label _label)
    (:`Update`
      (if (`self.firstTurntableUpdate`)
        (`SceneComponent.K2_SetWorldRotation` (`/EzCameraController/BP_turntableActor.DefaultSceneRoot` (`self.turnatableCameraObject`)) (`KismetMathLibrary.MakeRotator` 0.0 0.0 (.x _newtrack_0)) false false)
        (set `self.firstTurntableUpdate` false)
        (`KismetSystemLibrary.Delay` howLongToDoItFor)
        (set `self.turnTableRotating` false)
        (`self.stopTurnTable`)
        (else
          (`SceneComponent.K2_SetWorldRotation` (`/EzCameraController/BP_turntableActor.DefaultSceneRoot` (`self.turnatableCameraObject`)) (`KismetMathLibrary.MakeRotator` 0.0 0.0 (.x _newtrack_0)) false false))))
    (:`Finished`)))

(event `stopTurnTable`
  ; rotates the cameras parent in a circle rotating the camera around the center of the object to show off whatever is in view from all angles
  (if (stale `turnTableRotate` switchToPlayerCamera)
    (`self.changeBackToPlayerCamera`)
    (else
      (`/Engine/EditorBlueprintResources/StandardMacros.IsValid` (stale `turnTableRotate` cameraToSwitchBackTo)
        (:`Is Valid`
          (`self.changeToNewCamera` (stale `turnTableRotate` cameraToSwitchBackTo))))))
  (if (stale `turnTableRotate` disablePlayerInput)
    (`self.enablePlayerInput`)
    (goto _label :!via `Stop`)
    (else
      (goto _label :!via `Stop`))))

(event `lookAtPlayer`
  ; checks if the camera should be rotating to the player then does it if so
  (if (`self.rotateToPlayer`)
    (`SceneComponent.K2_SetWorldRotation` (`self.currentCamera`) (`KismetMathLibrary.FindLookAtRotation` (`SceneComponent.K2_GetComponentLocation` (`self.currentCamera`)) (`SceneComponent.K2_GetComponentLocation` (`Character.CapsuleComponent` (`self.playerCharacter`)))) false false)))

(event `shakeCameraPerlin`
  (params (duration :type "Float (double-precision)") (scale :type "Float (double-precision)"))
  ; shakes camera using diffrent shake patterns
  (`PlayerCameraManager.StartCameraShake` :`self` (`PlayerController.PlayerCameraManager` (`self.playerController`)) :`ShakeClass` "/EzCameraController/BP_cameraShakeperlinNoise.BP_cameraShakeperlinNoise_C" :`Scale` scale)
  (`KismetSystemLibrary.Delay` duration)
  (`PlayerCameraManager.StopCameraShake` (`PlayerController.PlayerCameraManager` (`self.playerController`)) null true))

(event `shakeCameraComposite`
  (params (duration :type "Float (double-precision)") (scale :type "Float (double-precision)"))
  ; shakes camera using diffrent shake patterns
  (`PlayerCameraManager.StartCameraShake` :`self` (`PlayerController.PlayerCameraManager` (`self.playerController`)) :`ShakeClass` "/EzCameraController/BP_cameraShakeCompisite.BP_cameraShakeCompisite_C" :`Scale` scale)
  (`KismetSystemLibrary.Delay` duration)
  (`PlayerCameraManager.StopCameraShake` (`PlayerController.PlayerCameraManager` (`self.playerController`)) null true))

(event `shakeCameraOscillator`
  (params (duration :type "Float (double-precision)") (scale :type "Float (double-precision)"))
  ; shakes camera using diffrent shake patterns
  (`PlayerCameraManager.StartCameraShake` :`self` (`PlayerController.PlayerCameraManager` (`self.playerController`)) :`ShakeClass` "/EzCameraController/BP_cameraShakeOscillator.BP_cameraShakeOscillator_C" :`Scale` scale)
  (`KismetSystemLibrary.Delay` duration)
  (`PlayerCameraManager.StopCameraShake` (`PlayerController.PlayerCameraManager` (`self.playerController`)) null true))

(event `shakeCameraSequence`
  (params (duration :type "Float (double-precision)") (scale :type "Float (double-precision)"))
  ; shakes camera using diffrent shake patterns
  (`PlayerCameraManager.StartCameraShake` :`self` (`PlayerController.PlayerCameraManager` (`self.playerController`)) :`ShakeClass` "/EzCameraController/BP_cameraShakeSequence.BP_cameraShakeSequence_C" :`Scale` scale)
  (`KismetSystemLibrary.Delay` duration)
  (`PlayerCameraManager.StopCameraShake` (`PlayerController.PlayerCameraManager` (`self.playerController`)) null true))

(event `disablePlayerInput`
  ; enable and disable player input
  (`self.DisableInput` (`self.playerCharacter`) (`self.playerController`)))

(event `enablePlayerInput`
  ; enable and disable player input
  (`self.EnableInput` (`self.playerCharacter`) (`self.playerController`)))

(fn `attatchCameraToSpringArm`
  (bind _springarm (`self.springArm`))
  ; attaches the camera to the players spring arm
  (`/Engine/EditorBlueprintResources/StandardMacros.IsValid` _springarm
    (:`Is Valid`
      (`SceneComponent.K2_AttachToComponent` (`self.playerCamera`) _springarm "None" "SnapToTarget" "SnapToTarget" "KeepWorld" true))))

(fn `changeBackToPlayerCamera`
  ; changes the current camera back to the player camera
  (`PlayerController.SetViewTargetWithBlend` (`self.playerController`) (`GameplayStatics.GetPlayerPawn` 0) 0.0 "VTBlend_Linear" 0.0 false)
  (set `self.turnTableRotating` false)
  (set `self.currentCamera` (`self.playerCamera`)))

(fn `changeToAndRotateTurntableCamera`
  (params (turnatableCameraObject :type "/EzCameraController/BP_turntableActor Object Reference") (howManyCirclesItWillCompleteInASecond :type "Float (double-precision)") (howLongToRotate :type "Float (double-precision)") (changeBackToPlayerCamera :type Boolean) (nonePlayerCameraToChangeBackTo :type "CameraComponent Object Reference") (disablePlayerInput :type Boolean))
  ; changes the current camera to a new one and then starts the turntable rotation of the said camera
  (if disablePlayerInput
    (`self.disablePlayerInput`))
  (set `self.turnatableCameraObject` turnatableCameraObject)
  (`PlayerController.SetViewTargetWithBlend` (`self.playerController`) turnatableCameraObject 0.0 "VTBlend_Linear" 0.0 false)
  (set `self.turnTableRotating` true)
  (set `self.firstTurntableUpdate` true)
  (`self.turnTableRotate` howManyCirclesItWillCompleteInASecond howLongToRotate nonePlayerCameraToChangeBackTo changeBackToPlayerCamera disablePlayerInput))

(fn `changeToNewCamera`
  (params (cameraToPoses :type "CameraComponent Object Reference"))
  ; chages current camera to a new one
  (`PlayerController.SetViewTargetWithBlend` (`self.playerController`) (`ActorComponent.GetOwner` cameraToPoses) 0.0 "VTBlend_Linear" 0.0 false)
  (set `self.turnTableRotating` false)
  (set `self.currentCamera` cameraToPoses))

(fn `detatchCamera`
  ; detatches the camera from the current object it is attached to
  (`SceneComponent.K2_DetachFromComponent` (`self.playerCamera`) "KeepWorld" "KeepWorld" "KeepWorld" true))

(fn `rotateCamera`
  (params (newRotation :type "Rotator Structure"))
  ; sets the roation of the camera
  (`SceneComponent.K2_SetWorldRotation` (`self.currentCamera`) newRotation false false))

(fn `rotatePlayeSpringArm`
  (params (newRotation :type "Rotator Structure"))
  ; rotates the spring arm if the reference to it isnt null
  (`/Engine/EditorBlueprintResources/StandardMacros.IsValid` (`self.springArm`)
    (:`Is Valid`
      (`SceneComponent.K2_SetWorldRotation` (`self.springArm`) newRotation false false))))

(fn `teleportCameraToPos`
  (params (position :type "Vector Structure"))
  ; instantly moves the camera to a new position
  (`SceneComponent.K2_SetWorldLocation` (`self.playerCamera`) position false false))

(fn `toggleConstantlyRotateToPlayer`
  ; starts rotating the camera to look at the player
  (if (`self.rotateToPlayer`)
    (set `self.rotateToPlayer` false)
    (if (`self.timerForLookingAtPlayerSetUp`)
      (`KismetSystemLibrary.K2_PauseTimerHandle` (`self.lookAtPlayerTimer`)))
    (else
      (set `self.rotateToPlayer` true)
      (if (`self.timerForLookingAtPlayerSetUp`)
        (`KismetSystemLibrary.K2_UnPauseTimerHandle` (`self.lookAtPlayerTimer`))
        (else
          (bind _returnvalue (`KismetSystemLibrary.K2_SetTimer` null "lookAtPlayer" 1e-06 true true))
          (set `self.lookAtPlayerTimer` _returnvalue)
          (set `self.timerForLookingAtPlayerSetUp` true))))))

(fn `UserConstructionScript`)